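; BP_EnemyActor is an enemy that can collide with the player's airplane or be killed for score.
; ChangeActorMaterial swaps the static mesh material according to the remaining health passed in.
; HitTargetActor checks for BP_AirPlane, damages the first airplane found in the level, and destroys the enemy.
; EnemyDie spawns a BP_3DAddScore at its Scene transform, awarding more for large enemies, then destroys itself.
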(event `self.ChangeActorMaterial`
  (params (InputHealth :type Integer))
  (bind _staticmesh (`self.StaticMesh`))
  (if (== InputHealth 2)
    (`PrimitiveComponent.SetMaterial` _staticmesh 0 "/Engine/VREditor/UI/DiscMaterial.DiscMaterial")
    (elif (== InputHealth 1)
      (`PrimitiveComponent.SetMaterial` _staticmesh 0 "/MeshModelingToolset/Materials/BrushIndicatorMaterial.BrushIndicatorMaterial"))))

(event `self.HitTargetActor`
  (params (TargetActor :type "Actor Object Reference"))
  (if (== (`GameplayStatics.GetObjectClass` TargetActor) "/Game/Blueprints/BP_AirPlane.BP_AirPlane_C")
    (bind _outactors (`GameplayStatics.GetAllActorsOfClass` "/Game/Blueprints/BP_AirPlane.BP_AirPlane_C"))
    (`/Game/Blueprints/BP_AirPlane.TakeDamage` (`|GetArrayItem` _outactors) 2.0)
    (`KismetSystemLibrary.PrintString` "Enemy Hit destory" false)
    (`self.K2_DestroyActor`)))

(event `self.EnemyDie`
  (bind _returnvalue (`|SpawnActorFromClass` "/Game/Blueprints/BP_3DAddScore.BP_3DAddScore_C" (`SceneComponent.K2_GetComponentToWorld` (`self.Scene`)) "Undefined" "OverrideRootScale" null null))
  (bind _returnvalue_2 (`self.GetIsLarge`))
  (`/Game/Blueprints/BP_3DAddScore.SetScore` _returnvalue (`KismetMathLibrary.SelectInt` 3 1 _returnvalue_2))
  (`self.K2_DestroyActor`))

(fn `UserConstructionScript`)