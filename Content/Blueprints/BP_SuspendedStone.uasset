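; BP_SuspendedStone is a short-lived floating stone actor that bobs vertically and destroys itself after a random lifetime.
; After a random startup delay, BeginPlay picks a mesh from MeshArray and sets a rotation from a fixed-seed stream.
; BeginShow loops through a FlipFlop that alternates the UpDown timeline forward and reverse, adding randomly scaled local Z offsets each update.
; CurrentLocation is stored on each swing but never read.
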(event `DelayDestroy`
  (`KismetSystemLibrary.Delay` (`KismetMathLibrary.RandomFloatInRange` 15.0 30.0))
  (`self.K2_DestroyActor`))

(event `BeginShow`
  (bind _returnvalue (`self.K2_GetActorLocation`))
  (`/Engine/EditorBlueprintResources/StandardMacros.FlipFlop`
    (:`A`
      (set `self.CurrentLocation` _returnvalue)
      (bind (_direction _track1) (`Timeline|UpDown` :!via `PlayFromStart` :!label _label)
        (:`Update`
          (`self.K2_AddActorLocalOffset` (`KismetMathLibrary.MakeVector` 0.0 0.0 (* _track1 (`KismetMathLibrary.RandomFloatInRange` 0.5 4.0)))))
        (:`Finished`
          (`self.BeginShow`))))
    (:`B`
      (set `self.CurrentLocation` _returnvalue)
      (goto _label :!via `ReverseFromEnd`))))

(event `self.ReceiveBeginPlay`
  (bind _mesharray (`self.MeshArray`))
  (`KismetSystemLibrary.Delay` (`KismetMathLibrary.RandomFloatInRange` 0.0 1.0))
  (`StaticMeshComponent.SetStaticMesh` (`self.StaticMesh`) (`|GetArrayItem` _mesharray (`KismetMathLibrary.RandomIntegerInRange` 0 (- (`KismetArrayLibrary.Array_Length` _mesharray) 1))))
  (`self.BeginShow`)
  (`self.DelayDestroy`)
  (`SceneComponent.K2_SetRelativeRotation` (`self.StaticMesh`) (`KismetMathLibrary.RandomRotatorFromStream` true (`KismetMathLibrary.MakeRandomStream` 1)) false false))

(fn `UserConstructionScript`)