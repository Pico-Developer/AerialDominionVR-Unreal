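; BP_UIActor is an actor that hosts UI through a widget component.
; Custom events swap the displayed widget and set its draw size, while UIInit finds the first existing UI_MainInfo widget and calls UIShow on it.
; Tick polls GradesManagerSubsystem for the GamePlaying status and checks HiddenInPlaying once through a DoOnce, though that branch currently performs no action.
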(event `ChangeUMG`
  (params (Widget :type "UserWidget Object Reference"))
  (`WidgetComponent.SetWidget` (`self.Widget`) Widget))

(event `SetDrawSize`
  (params (Size :type "Vector2D Structure"))
  (`WidgetComponent.SetDrawSize` (`self.Widget`) Size))

(event `UIInit`
  (bind _foundwidgets (`WidgetBlueprintLibrary.GetAllWidgetsOfClass` "/Game/UMG/UI_MainInfo.UI_MainInfo_C" false))
  (bind _output (`|GetArrayItem` _foundwidgets))
  (`/Engine/EditorBlueprintResources/StandardMacros.IsValid` _output
    (:`Is Valid`
      (`/Game/UMG/UI_MainInfo.UIShow` _output))))

(event `self.ReceiveTick`
  (params (DeltaSeconds :type "Float (single-precision)"))
  (bind _returnvalue (`GradesManagerSubsystem.GetGameStatus` (subsystem `GradesManagerSubsystem`)))
  (if (`|EnumEquality` _returnvalue "GamePlaying")
    (`/Engine/EditorBlueprintResources/StandardMacros.DoOnce` false
      (:`Completed`
        (if (`self.bHiddenInPlaying`)
          _)))))

(fn `UserConstructionScript`)