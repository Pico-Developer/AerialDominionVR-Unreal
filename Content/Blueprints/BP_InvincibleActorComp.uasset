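; BP_InvincibleActorComp is a protective invincibility actor that attaches to the airplane and destroys enemy threats that touch it.
; AttachandInvincibleTarget finds the first BP_AirPlane, teleports to it and snap-attaches so the protection follows the plane.
; Its static mesh overlap event casts the other actor to BP_EnemyBullet, then BP_EnemyActor, destroying either and printing a debug message.
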(event `self.AttachAndInvincibleTarget`
  (bind _outactors (`GameplayStatics.GetAllActorsOfClass` "/Game/Blueprints/BP_AirPlane.BP_AirPlane_C"))
  (bind _output (`|GetArrayItem` _outactors))
  (`/Engine/EditorBlueprintResources/StandardMacros.IsValid` _output
    (:`Is Valid`
      (`self.K2_SetActorLocation` (`self.K2_GetActorLocation` _output) false true)
      (`self.K2_AttachToActor` _output "None" "SnapToTarget" "SnapToTarget" "SnapToTarget"))))

(event `self.StaticMeshComp.OnComponentBeginOverlap`
  (params (OverlappedComponent :type "PrimitiveComponent Object Reference") (OtherActor :type "Actor Object Reference") (OtherComp :type "PrimitiveComponent Object Reference") (OtherBodyIndex :type Integer) (bFromSweep :type Boolean) (SweepResult :type "HitResult Structure (by ref)"))
  (bind _asbp_enemy_bullet (cast `/Game/Blueprints/BP_EnemyBullet` OtherActor)
    (:`then`
      (`KismetSystemLibrary.PrintString` "Protuct destroy" false)
      (`self.K2_DestroyActor` _asbp_enemy_bullet))
    (:`CastFailed`
      (bind _asbp_enemy_actor (cast `/Game/Blueprints/BP_EnemyActor` OtherActor))
      (`KismetSystemLibrary.PrintString` "Protuct destroy" false)
      (`self.K2_DestroyActor` _asbp_enemy_actor))))

(fn `UserConstructionScript`)