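; VR player pawn for a Pico airplane shooter that spawns a BP_AirPlane attached to its SMR component.
; Right trigger clicks widgets and, during play, fires bullets with sound from the Arrow; the right A button calls the game mode's pause.
; Each tick the right joystick scrolls widgets and a forward trace, ignoring airplanes, stretches TraceMesh into a laser pointer ending at the hit or maximum range.
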(event `self.ReceiveBeginPlay`
  (`HeadMountedDisplayFunctionLibrary.SetTrackingOrigin` "Floor")
  (bind _returnvalue (`|SpawnActorFromClass` "/Game/Blueprints/BP_AirPlane.BP_AirPlane_C" (`SceneComponent.K2_GetComponentToWorld` (`self.SM_R`)) "Undefined" "OverrideRootScale" null null))
  (bind _output_get (set `self.AirPlane` _returnvalue))
  (`self.K2_AttachToComponent` _output_get (`self.SM_R`) "None" "SnapToTarget" "SnapToTarget" "SnapToTarget" true))

(event `self.ReceiveTick`
  (params (DeltaSeconds :type "Float (single-precision)"))
  (set `self.PlaneLocation` (`SceneComponent.K2_GetComponentLocation` (`self.SM_R`)))
  (`WidgetInteractionComponent.ScrollWheel` (`self.WidgetInteraction`) (`self.GetInputAxisValue`))
  (`self.RightHandTrace`))

(event `InputAction|Pico_Trigger_R`
  (params (Key :type "Key Structure"))
  (bind _arrow (`self.Arrow`))
  (:`Pressed`
    (`WidgetInteractionComponent.PressPointerKey` (`self.WidgetInteraction`) "LeftMouseButton")
    (bind _returnvalue (`GradesManagerSubsystem.GetGameStatus` (subsystem `GradesManagerSubsystem`)))
    (if (`|EnumEquality` _returnvalue "GamePlaying")
      (`|SpawnActorFromClass` "/Game/Blueprints/BP_PlayerBullet.BP_PlayerBullet_C" (`SceneComponent.K2_GetComponentToWorld` _arrow) "Undefined" "OverrideRootScale" null null)
      (`GameplayStatics.PlaySoundAtLocation` "/Game/MobileStarterContent/Audio/Explosion02_Cue.Explosion02_Cue" (`SceneComponent.K2_GetComponentLocation` _arrow) (struct) 1.0 1.0 0.0 null null null)))
  (:`Released`
    (`WidgetInteractionComponent.ReleasePointerKey` (`self.WidgetInteraction`) "LeftMouseButton")))

(event `InputAction|Pico_Trigger_R`
  (params (Key :type "Key Structure")))

(event `InputAction|Pico_A_R`
  (params (Key :type "Key Structure"))
  (:`Pressed`
    (bind _asbp_aeial_dominion_gm (cast `/Game/Blueprints/BP_AeialDominionGM` (`GameplayStatics.GetGameMode`)))
    (`/Game/Blueprints/BP_AeialDominionGM.GamePause` _asbp_aeial_dominion_gm)))

(fn `RightHandTrace`
  (bind _returnvalue (`SceneComponent.K2_GetComponentLocation` (`self.Arrow`)))
  (bind _returnvalue_2 (+ _returnvalue (* (`SceneComponent.GetForwardVector` (`self.Arrow`)) 1000)))
  (bind _outactors (`GameplayStatics.GetAllActorsOfClass` "/Game/Blueprints/BP_AirPlane.BP_AirPlane_C"))
  (bind (_outhit _returnvalue_3) (`KismetSystemLibrary.LineTraceSingle` _returnvalue _returnvalue_2 "TraceTypeQuery1" false _outactors "None" true (struct :`R` 1.0 :`A` 1.0) (struct :`G` 1.0 :`A` 1.0) 0.0))
  (bind (_bblockinghit _binitialoverlap _time _distance _location) (`GameplayStatics.BreakHitResult` _outhit))
  (`self.TraceAdaption` _returnvalue_2 _returnvalue _location _returnvalue_3 _distance))

(fn `TraceAdaption`
  (params (EndLocation :type "Vector Structure") (StartLocation :type "Vector Structure") (HitLocation :type "Vector Structure") (bIsHit :type Boolean) (Distance :type "Float (double-precision)"))
  (bind _tracemesh (`self.TraceMesh`))
  (`SceneComponent.K2_SetWorldLocation` _tracemesh (/ (+ (`KismetMathLibrary.SelectVector` HitLocation EndLocation bIsHit) StartLocation) 2) false true)
  (`SceneComponent.SetWorldScale3D` _tracemesh (`KismetMathLibrary.MakeVector` 0.001 0.001 (/ (`KismetMathLibrary.SelectFloat` Distance 1000.0 bIsHit) 100.0))))

(fn `UserConstructionScript`)