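; Game mode Blueprint for Aerial Dominion that handles game end, pausing and PICO platform achievement and leaderboard calls.
; Game end and pause toggle tagged BP_UIActor panels, with game end also showing game-over and refreshing achievement and leaderboard widgets after a delay.
; Pause state lives in GradesManagerSubsystem.
; Separate events unlock or increment achievements and write scores to the PicoWorld leaderboard, with async callbacks logging results to that subsystem.
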(event `self.CallGameEnd`
  (`|ExecutionSequence`
    (:`then_0`
      (`self.VisibleDefaultUI` true))
    (:`then_1`
      (bind _outactors (`GameplayStatics.GetAllActorsOfClassWithTag` "/Game/Blueprints/BP_UIActor.BP_UIActor_C" "MainInfo"))
      (bind _output (`|GetArrayItem` _outactors))
      (`/Engine/EditorBlueprintResources/StandardMacros.IsValid` _output
        (:`Is Valid`
          (`/Game/Blueprints/BP_UIActor.UIInit` _output)
          (`self.SetActorEnableCollision` _output true)
          (`self.SetActorHiddenInGame` _output false)
          (bind _foundwidgets (`WidgetBlueprintLibrary.GetAllWidgetsOfClass` "/Game/UMG/UI_MainInfo.UI_MainInfo_C" false))
          (bind _output_2 (`|GetArrayItem` _foundwidgets))
          (`/Engine/EditorBlueprintResources/StandardMacros.IsValid` _output_2
            (:`Is Valid`
              (`/Game/UMG/UI_MainInfo.GameOverShow` _output_2))))))
    (:`then_2`
      (`KismetSystemLibrary.Delay` 1.0)
      (bind _foundwidgets_2 (`WidgetBlueprintLibrary.GetAllWidgetsOfClass` "/Game/UMG/UI_Achievements.UI_Achievements_C" false))
      (bind _output_3 (`|GetArrayItem` _foundwidgets_2))
      (`/Engine/EditorBlueprintResources/StandardMacros.IsValid` _output_3
        (:`Is Valid`
          (`/Game/UMG/UI_Achievements.AchievementRefresh` _output_3))))
    (:`then_3`
      (`KismetSystemLibrary.Delay` 1.0)
      (bind _foundwidgets_3 (`WidgetBlueprintLibrary.GetAllWidgetsOfClass` "/Game/UMG/UI_LeaderBoardForALL.UI_LeaderBoardForAll_C" false))
      (bind _output_4 (`|GetArrayItem` _foundwidgets_3))
      (`/Engine/EditorBlueprintResources/StandardMacros.IsValid` _output_4
        (:`Is Valid`
          (`/Game/UMG/UI_LeaderBoardForALL.LeaderBoardRefresh` _output_4))))))

(event `self.UnLockTargetAchievements`
  (params (InAchName :type String))
  (`OnlinePicoAchievementsFunction.PicoUnlock` InAchName "" (delegate `OnAchievementUnLock`)))

(event `OnAchievementUnLock`
  (params (bIsError :type Boolean) (ErrorMessage :type String) (AchievementUpdate :type "Pico_AchievementUpdate Object Reference"))
  (bind _returnvalue (subsystem `GradesManagerSubsystem`))
  (if bIsError
    (`GradesManagerSubsystem.SetLogString` _returnvalue (`KismetStringLibrary.Concat_StrStr` "OnAchievementUnLockError: " ErrorMessage))
    (else
      (`GradesManagerSubsystem.SetLogString` _returnvalue (`KismetStringLibrary.Concat_StrStr` "OnAchievementUnLockSuccessed:  Ach Name:" (`Pico_AchievementUpdate.GetName` AchievementUpdate))))))

(event `self.WriteLeaderboardEntry`
  (params (InTotalScore :type "Float (single-precision)"))
  (`OnlinePicoLeaderboardsFunction.WriteEntry` "PicoWorld" (`KismetStringLibrary.Conv_DoubleToString` InTotalScore) "" false (delegate `OnWriteLeaderComplete`)))

(event `OnWriteLeaderComplete`
  (params (bIsError :type Boolean) (ErrorMessage :type String) (WriteResult :type Boolean))
  (bind _returnvalue (subsystem `GradesManagerSubsystem`))
  (if bIsError
    (`GradesManagerSubsystem.SetLogString` _returnvalue (`KismetStringLibrary.Concat_StrStr` "WriteLeaderEntry Failed:" ErrorMessage))
    (else
      (`GradesManagerSubsystem.SetLogString` _returnvalue (`KismetStringLibrary.Concat_StrStr` "WriteLeaderEntry Successed: result:" (`KismetStringLibrary.Conv_BoolToString` WriteResult))))))

(event `self.AddCountAchievements`
  (`OnlinePicoAchievementsFunction.PicoAddCount` "FullFirepower" "1" "" (delegate `OnAddCoutComplete`))
  (`OnlinePicoAchievementsFunction.PicoAddCount` "Unstoppable" "1" "" (delegate `OnAddCoutComplete`))
  (`OnlinePicoAchievementsFunction.PicoAddCount` "BossSlayer" "1" "" (delegate `OnAddCoutComplete`)))

(event `OnAddCoutComplete`
  (params (bIsError :type Boolean) (ErrorMessage :type String) (AchievementUpdate :type "Pico_AchievementUpdate Object Reference"))
  (bind _returnvalue (subsystem `GradesManagerSubsystem`))
  (if bIsError
    (`GradesManagerSubsystem.SetLogString` _returnvalue (`KismetStringLibrary.Concat_StrStr` "OnAddCoutComplete Error: " ErrorMessage))
    (else
      (`GradesManagerSubsystem.SetLogString` _returnvalue (`KismetStringLibrary.Concat_StrStr` "OnAddCoutComplete Successedr:  Ach Name:" (`Pico_AchievementUpdate.GetName` AchievementUpdate))))))

(event `GamePause`
  (bind _returnvalue (subsystem `GradesManagerSubsystem`))
  (bind _returnvalue_2 (`GradesManagerSubsystem.GetGameStatus` _returnvalue))
  (if (`|EnumEquality` _returnvalue_2 "GamePlaying")
    (`GradesManagerSubsystem.GamePause` _returnvalue true)
    (`self.VisibleDefaultUI` true)
    (elif (`|EnumEquality` _returnvalue_2 "GamePause")
      (`GradesManagerSubsystem.GamePause` _returnvalue false)
      (`self.VisibleDefaultUI` false))))

(event `VisibleDefaultUI`
  (params (IsVisable :type Boolean))
  (bind _outactors (`GameplayStatics.GetAllActorsOfClass` "/Game/Blueprints/BP_UIActor.BP_UIActor_C"))
  (for _array_element _outactors
    (if (`self.ActorHasTag` _array_element "MainInfo")
      (`self.SetActorHiddenInGame` _array_element (not IsVisable))
      (`self.SetActorEnableCollision` _array_element IsVisable)
      (if IsVisable
        (`/Game/Blueprints/BP_UIActor.UIInit` _array_element))
      (elif (or (`self.ActorHasTag` _array_element "Leaderboards") (`self.ActorHasTag` _array_element "Achievements"))
        (`self.SetActorHiddenInGame` _array_element (not IsVisable))
        (`self.SetActorEnableCollision` _array_element IsVisable)))))

(fn `UserConstructionScript`)