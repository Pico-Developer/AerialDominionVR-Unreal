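; BP_EnemyBullet is an enemy projectile that damages the player's airplane.
; It destroys itself two seconds after BeginPlay.
; When HitTargetActor reports a target of exactly the BP_AirPlane class, it deals one point of damage to it and destroys itself.
; Its own collision overlap handler is empty, and nothing in this graph calls HitTargetActor.
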(event `self.ReceiveBeginPlay`
  (`KismetSystemLibrary.Delay` 2.0)
  (`self.K2_DestroyActor`))

(event `self.HitTargetActor`
  (params (TargetActor :type "Actor Object Reference"))
  (if (== (`GameplayStatics.GetObjectClass` TargetActor) "/Game/Blueprints/BP_AirPlane.BP_AirPlane_C")
    (bind _asbp_air_plane (cast `/Game/Blueprints/BP_AirPlane` TargetActor))
    (`/Engine/EditorBlueprintResources/StandardMacros.IsValid` _asbp_air_plane
      (:`Is Valid`
        (`/Game/Blueprints/BP_AirPlane.TakeDamage` _asbp_air_plane 1.0)
        (`KismetSystemLibrary.PrintString` "EnemyBullet destroy" false)
        (`self.K2_DestroyActor`)))))

(event `self.CollisionComponent.OnComponentBeginOverlap`
  (params (OverlappedComponent :type "PrimitiveComponent Object Reference") (OtherActor :type "Actor Object Reference") (OtherComp :type "PrimitiveComponent Object Reference") (OtherBodyIndex :type Integer) (bFromSweep :type Boolean) (SweepResult :type "HitResult Structure (by ref)")))

(fn `UserConstructionScript`)