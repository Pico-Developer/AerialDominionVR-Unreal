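; BP_PlayerBullet is the player's projectile, which damages the first enemy it touches and then destroys itself.
; Tick polls the collision component for overlapping BP_EnemyActor instances and passes InputDamage to the first one through OnDamageReveived.
; BeginPlay starts a short delay that destroys bullets still alive when it ends.
; The HitTargetActor event is empty, and an enemy class-check branch is left unconnected.
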(event `self.ReceiveBeginPlay`
  (`KismetSystemLibrary.Delay` 2.0)
  (`self.K2_DestroyActor`))

(event `self.HitTargetActor`
  (params (TargetActor :type "Actor Object Reference")))

(event `self.ReceiveTick`
  (params (DeltaSeconds :type "Float (single-precision)"))
  (bind _overlappingactors (`PrimitiveComponent.GetOverlappingActors` (`self.CollisionComponent`) "/Game/Blueprints/BP_EnemyActor.BP_EnemyActor_C"))
  (bind _output (`|GetArrayItem` _overlappingactors))
  (if (> (`KismetArrayLibrary.Array_Length` _overlappingactors) 0)
    (`/Engine/EditorBlueprintResources/StandardMacros.IsValid` _output
      (:`Is Valid`
        (bind _asbp_enemy_actor (cast `/Game/Blueprints/BP_EnemyActor` _output))
        (`EnemyActor.OnDamageReveived` _asbp_enemy_actor (`self.Input Damage`))
        (`KismetSystemLibrary.PrintString` "PlayerBullet destroy" false)
        (`self.K2_DestroyActor`)))))

(fn `UserConstructionScript`)